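; Floating status text actor in the damage display system that shows colored text moving vertically, then destroys itself after covering a set distance.
; On initialization it passes text and color to a scalable text widget and computes the per-tick displacement, or warns if the widget class is incompatible.
; It overrides the parent's location update to step along Z, estimates distance from tick count, and reports when the max-scale point is passed.
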(event `self.ReceiveBeginPlay`
  (`parent.ReceiveBeginPlay`))

(event `self.ReceiveTick`
  (params (DeltaSeconds :type "Float (single-precision)"))
  (`parent.ReceiveTick` DeltaSeconds)
  (if (>= (`self.GetVerticalDistanceCovered`) (`self.DistanceToCover`))
    (`self.K2_DestroyActor`)))

(event `self.RunInitializationProtocols`
  (bind _aswidget_scalable_text_display (cast `/Game/DamageDisplaySystem/UI/Widget_ScalableTextDisplay` (`WidgetComponent.GetUserWidgetObject` (`self.TextDisplayWidgetComponent`))) ; Evaluates the widget class at the start before activating text display
    (:`then`
      (`/Game/DamageDisplaySystem/UI/Widget_ScalableTextDisplay.SetDisplayText` _aswidget_scalable_text_display (`self.StatusText`) (`self.TextColor`))
      (`self.SetLinearMotionConstraints`)
      (`parent.RunInitializationProtocols`))
    (:`CastFailed`
      (`self.DisplayWidgetIncompatibilityWarning`))))

(event `self.UpdateWidgetLocation`
  (bind (_returnvalue_x _returnvalue_y _returnvalue_z) (`KismetMathLibrary.BreakVector` (`self.K2_GetActorLocation`)))
  (`self.K2_SetActorLocation` (`KismetMathLibrary.MakeVector` _returnvalue_x _returnvalue_y (+ _returnvalue_z (`self.VerticalDisplacementPerTick`)))))

(fn `CalculateVerticalMovementPerTick`
  (returns (ReturnValue :type "Float (double-precision)"))
  (return (* (`self.DistanceToCover`) (`self.MovementSpeedController`))))

(fn `GetVerticalDistanceCovered`
  (returns (ReturnValue :type "Float (double-precision)"))
  (return (* (`self.CurrentTickCount`) (`KismetMathLibrary.Abs` (`self.VerticalDisplacementPerTick`)))))

(fn `ReachedPointOfMaxWidgetScale?`
  (returns (`Yes?` :type Boolean))
  (return (> (`self.GetVerticalDistanceCovered`) (* (`self.DistanceToCover`) (`self.%DistanceToPointOfMaxScale`)))))

(fn `SetLinearMotionConstraints`
  ;[0 1 0 0.5] Sets the movement constraints along the linear path
  (set `self.VerticalDisplacementPerTick` (`self.CalculateVerticalMovementPerTick`))
  (return))

(fn `UserConstructionScript`)