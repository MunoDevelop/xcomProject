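; Actor component that rolls damage values and can show them as floating text actors at its owner.
; PerformDamageAssessment scales base damage by a random modifier, applies a percentage-chance critical multiplier, and returns the final damage and crit flag without applying them.
; When display is enabled, it spawns a damage text actor with the truncated value at an offset from the owner, plus a status text actor on critical hits.
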(fn `CalculateDamage`
  (params (BaseDamage :type "Float (double-precision)") (MinDamageModifier :type "Float (double-precision)") (MaxDamageModifier :type "Float (double-precision)") (CritChance :type "Float (double-precision)") (CritDamageModifier :type "Float (double-precision)"))
  (returns (FinalDamage :type "Float (double-precision)") (`IsACritHit?` :type Boolean))
  (locals (Local_CurrentDamage :type "Float (double-precision)") (`Local_IsACritHit?` :type Boolean :default false))
  ;[0 1 1 0.5] Calculates the final damage received & returns the information
  (set `local.Local_CurrentDamage` (* BaseDamage (`KismetMathLibrary.RandomFloatInRange` MinDamageModifier MaxDamageModifier)))
  (if (< (`KismetMathLibrary.RandomFloatInRange` 0.0 100.0) CritChance)
    (set `local.Local_IsACritHit?` true)
    (set `local.Local_CurrentDamage` (* (`local.Local_CurrentDamage`) CritDamageModifier))
    (else
      (set `local.Local_IsACritHit?` false)))
  (return (`local.Local_CurrentDamage`) (`local.Local_IsACritHit?`)))

(fn `DisplayDamageTexts`
  (params (FinalDamage :type "Float (double-precision)") (`IsACritHit?` :type Boolean))
  (bind _returnvalue (`KismetMathLibrary.Conv_VectorToTransform` (+ (`Actor.K2_GetActorLocation` (`self.GetOwner`)) (`self.DamageTextDisplaySpawnOffset`))))
  (`|SpawnActorFromClass` (`self.DamageTextDisplayActorClass`) _returnvalue "AlwaysSpawn" "OverrideRootScale" null (`KismetMathLibrary.FTrunc` FinalDamage) null) ; Spawns an actor to display the damage taken
  (if `IsACritHit?`
    (`|SpawnActorFromClass` (`self.StatusTextDisplayActorClass`) _returnvalue "AlwaysSpawn" "OverrideRootScale" null (`self.StatusText_CriticalHit`) null) ; Spawns an actor to display the critical hit status
  ))

(fn `PerformDamageAssessment`
  (params (BaseDamage :type "Float (double-precision)") (MinDamageModifier :type "Float (double-precision)") (MaxDamageModifier :type "Float (double-precision)") (CritChance :type "Float (double-precision)") (CritDamageModifier :type "Float (double-precision)"))
  (returns (FinalDamage :type "Float (double-precision)") (`IsACritHit?` :type Boolean))
  (bind (_finaldamage _isacrithit_) (`self.CalculateDamage` BaseDamage MinDamageModifier MaxDamageModifier CritChance CritDamageModifier)) ; Calculates final damage to be applied
  (if (`self.DisplayDamage?`)
    (`self.DisplayDamageTexts` _finaldamage _isacrithit_))
  (return _finaldamage _isacrithit_))