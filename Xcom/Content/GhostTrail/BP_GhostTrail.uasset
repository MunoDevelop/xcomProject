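; BP_GhostTrail is an actor that leaves a short-lived frozen copy of a skeletal mesh's pose, serving as one ghost in a trail.
; On BeginPlay it assigns the given mesh to a poseable mesh, swaps each material for a dynamic instance stored in MatList, and copies the source component's pose once.
; It destroys itself after TailLength seconds, with no material parameter changes in this graph.
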(event `self.ReceiveBeginPlay`
  (`SkinnedMeshComponent.SetSkinnedAssetAndUpdate` (`self.PoseableMesh`) (`self.skeletalMesh`) true)
  (for _ (`MeshComponent.GetMaterials` (`self.PoseableMesh`))
    (bind _returnvalue (`KismetMaterialLibrary.CreateDynamicMaterialInstance` null))
    (bind _returnvalue_2 (`KismetArrayLibrary.Array_Add` (`self.matList`) _returnvalue))
    (`PrimitiveComponent.SetMaterial` (`self.PoseableMesh`) _returnvalue_2 _returnvalue))
  (`PoseableMeshComponent.CopyPoseFromSkeletalComponent` (`self.PoseableMesh`) (`self.smComponent`))
  (`KismetSystemLibrary.Delay` (`self.tailLength`))
  (`self.K2_DestroyActor`))

(fn `UserConstructionScript`)