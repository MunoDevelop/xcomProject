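; EmitterBP is a placed emitter that fires one homing projectile when play begins.
; On BeginPlay it spawns a fire particle at its start offset, aimed along HommingDirection, then spawns a Particle_BP there with the same rotation.
; It hands that projectile the HomingTarget's mesh, homing start and blend times, and its trail and explosion particle templates.
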(event `self.ReceiveBeginPlay`
  (bind _returnvalue (`SceneComponent.K2_GetComponentRotation` (`self.hommingDirection`)))
  (bind _returnvalue_2 (+ (`self.K2_GetActorLocation`) (`self.startPoint`)))
  (`GameplayStatics.SpawnEmitterAtLocation` (`self.fireParticle`) _returnvalue_2 _returnvalue)
  (bind _returnvalue_3 (`|SpawnActorFromClass` "/Game/ParticleSystem/Particle_BP.Particle_BP_C" (`KismetMathLibrary.MakeTransform` _returnvalue_2 _returnvalue) "Undefined" "OverrideRootScale" null 2000.0 1000.0 4.0 null))
  (`/Game/ParticleSystem/Particle_BP.HomingMissile` _returnvalue_3 (`Character.Mesh` (`self.homingTarget`)) (`self.HomingStartTime`) 0.0 (`self.HomingBlendTime`))
  (`/Game/ParticleSystem/Particle_BP.Proj_PT_Set` _returnvalue_3 null (`self.movingParticle`) (`self.explosionParticle`) false))

(fn `UserConstructionScript`)