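; Utility function library for modular weapons that creates, reads and edits WeaponCode strings describing a weapon's type, parts and materials.
; Codes use the layout Type:Parts:Materials, with underscore-separated entries and parts written as prefix plus mesh index.
; Lookups read types, parts and material sets from WeaponData class defaults.
; Randomizers roll optional parts against a weight and can selectively keep an existing code's type, parts or materials.
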(fn `Available Weapon Parts of Type`
  (params (`Weapon Type` :type String) (`Exclude Optional Parts` :type Boolean))
  (returns (`Available Parts` :type "Array of String"))
  (locals (`Found Types` :type "Array of String") (`Local Weapon Parts` :type "Array of /Game/ModularWeapons/Data/WeaponPart Structure"))
  (bind _found_types (`local.Found Types`))
  (bind _output_get (set `local.Local Weapon Parts` (defaults `/Game/ModularWeapons/Data/WeaponData` "/Game/ModularWeapons/Data/WeaponData.WeaponData_C")))
  (for _array_element _output_get
    (bind (_weapontypename _partprefix _meshes _optional) (break `/Game/ModularWeapons/Data/WeaponPart` _array_element))
    (if (== `Weapon Type` _weapontypename)
      (if `Exclude Optional Parts`
        (if (not _optional)
          (bind _returnvalue (`KismetStringLibrary.ToLower` _partprefix))
          (if (not (`KismetArrayLibrary.Array_Contains` _found_types _returnvalue)) :!label _label
            (`KismetArrayLibrary.Array_AddUnique` _found_types _returnvalue)))
        (else
          (goto _label)))))
  (return (`local.Found Types`)))

(fn `Available Weapon Types`
  (returns (`Available Types` :type "Array of String"))
  (locals (`Found Types` :type "Array of String") (`Local Weapon Parts` :type "Array of /Game/ModularWeapons/Data/WeaponPart Structure"))
  (bind _found_types (`local.Found Types`))
  (bind _output_get (set `local.Local Weapon Parts` (defaults `/Game/ModularWeapons/Data/WeaponData` "/Game/ModularWeapons/Data/WeaponData.WeaponData_C")))
  (for _array_element _output_get
    (bind _returnvalue (`KismetStringLibrary.ToLower` (`.WeaponTypeName_15_FC0C2B194457E4D9BF092A8C7524DB41` (break `/Game/ModularWeapons/Data/WeaponPart` _array_element))))
    (if (not (`KismetArrayLibrary.Array_Contains` _found_types _returnvalue))
      (`KismetArrayLibrary.Array_AddUnique` _found_types _returnvalue)))
  (return (`local.Found Types`)))

(fn `Compile WeaponCode`
  (params (`Weapon Type` :type String) (`Weapon Parts` :type "Array of String") (`Weapon Materials` :type "Array of String"))
  (returns (WeaponCode :type String))
  (locals (`Local WeaponCode` :type String))
  (set `local.Local WeaponCode` `Weapon Type`)
  (for (_array_element _array_index) `Weapon Parts`
    (set `local.Local WeaponCode` (`KismetStringLibrary.Concat_StrStr` (`local.Local WeaponCode`) (`KismetMathLibrary.SelectString` ":" "_" (== _array_index 0)) _array_element)))
  (for (_array_element_2 _array_index_2) `Weapon Materials`
    (set `local.Local WeaponCode` (`KismetStringLibrary.Concat_StrStr` (`local.Local WeaponCode`) (`KismetMathLibrary.SelectString` ":" "_" (== _array_index_2 0)) _array_element_2)))
  (return (`local.Local WeaponCode`)))

(fn `Decompile WeaponCode`
  (params (`Weapon Code` :type String))
  (returns (`Weapon Type` :type String) (`Weapon Parts` :type "Array of String") (`Weapon Materials` :type "Array of String"))
  (locals (`Local WeaponParts` :type "Array of String") (`Local WeaponMats` :type "Array of String"))
  (set `local.Local WeaponParts` (`self.Get Parts from WeaponCode` `Weapon Code`))
  (set `local.Local WeaponMats` (`self.Get Materials from WeaponCode` `Weapon Code`))
  (return (`self.Get Type from WeaponCode` `Weapon Code`) (`local.Local WeaponParts`) (`local.Local WeaponMats`)))

(fn `Filter Weapon Parts by Type`
  (params (`Weapon Parts` :type "Array of /Game/ModularWeapons/Data/WeaponPart Structure") (`Weapon Type` :type String) (`Exclude Optional Parts` :type Boolean) (`Optional Parts Weight` :type "Float (double-precision)" :default 1.0))
  (returns (Parts :type "Array of /Game/ModularWeapons/Data/WeaponPart Structure"))
  (locals (`Parts Array` :type "Array of /Game/ModularWeapons/Data/WeaponPart Structure") (`Incoming Parts Array` :type "Array of /Game/ModularWeapons/Data/WeaponPart Structure"))
  (bind _output_get (set `local.Incoming Parts Array` `Weapon Parts`))
  (for _array_element _output_get
    (if `Exclude Optional Parts`
      (bind (_weapontypename _partprefix _meshes _optional) (break `/Game/ModularWeapons/Data/WeaponPart` _array_element))
      (bind _returnvalue (== _weapontypename `Weapon Type`))
      (bind _returnvalue_2 (not _optional))
      (if (and _returnvalue _returnvalue_2)
        (`KismetArrayLibrary.Array_AddUnique` (`local.Parts Array`) _array_element :!label _label))
      (elif (and _returnvalue _returnvalue_2)
        (goto _label)
        (elif (and _optional (>= `Optional Parts Weight` (`KismetMathLibrary.RandomFloat`)))
          (goto _label)))))
  (return (`local.Parts Array`)))

(fn `Get Materials from WeaponCode`
  (params (WeaponCode :type String))
  (returns (`Material ShortNames` :type "Array of String"))
  (locals (`Found Mats Array` :type "Array of String"))
  (bind _output_get (set `local.Found Mats Array` (`KismetStringLibrary.ParseIntoArray` (`KismetArrayLibrary.Array_Get` (`KismetStringLibrary.ParseIntoArray` WeaponCode ":") 2) "_")))
  (return _output_get))

(fn `Get MaterialSets of Slot`
  (params (Slot :type "/Game/ModularWeapons/Data/MaterialSlot Enum"))
  (returns (MaterialSets :type "Array of /Game/ModularWeapons/Data/MaterialSet Structure") (`MaterialSets ShortNames` :type "Array of String"))
  (locals (`Filtered Materials` :type "Array of /Game/ModularWeapons/Data/MaterialSet Structure") (`Filtered Material Strings` :type "Array of String") (`Unfiltered Materials` :type "Array of /Game/ModularWeapons/Data/MaterialSet Structure"))
  (bind _output_get (set `local.Unfiltered Materials` (`.MaterialSets` (defaults `/Game/ModularWeapons/Data/WeaponData` "/Game/ModularWeapons/Data/WeaponData.WeaponData_C"))))
  (for _array_element _output_get
    (bind ((`MaterialType_19_89702AAB40093D038C1E1890759BD0A6` _materialtype) (`MaterialUniqueShortName_27_054530BA4E6ABC3F1CEEC68FA6F3C425` _materialuniqueshortname)) (break `/Game/ModularWeapons/Data/MaterialSet` _array_element))
    (if (`|EnumEquality` _materialtype Slot)
      (`KismetArrayLibrary.Array_Add` (`local.Filtered Materials`) _array_element)
      (`KismetArrayLibrary.Array_Add` (`local.Filtered Material Strings`) _materialuniqueshortname)))
  (return (`local.Filtered Materials`) (`local.Filtered Material Strings`)))

(fn `Get MaterialSlots of WeaponType`
  (params (WeaponType :type String))
  (returns (Slots :type "Array of /Game/ModularWeapons/Data/MaterialSlot Enum"))
  (locals (`Material Slots` :type "Array of /Game/ModularWeapons/Data/MaterialSlot Enum") (`Local Weapon Types` :type "Array of /Game/ModularWeapons/Data/WeaponType Structure"))
  (bind _output_get (set `local.Local Weapon Types` (`.WeaponTypes` (defaults `/Game/ModularWeapons/Data/WeaponData` "/Game/ModularWeapons/Data/WeaponData.WeaponData_C"))))
  (for _array_element _output_get
    (bind (_weapontypename _materialslottypes) (break `/Game/ModularWeapons/Data/WeaponType` _array_element))
    (if (== WeaponType _weapontypename)
      (set `local.Material Slots` _materialslottypes)
      (break)))
  (return (`local.Material Slots`)))

(fn `Get Num MaterialSlots of WeaponType`
  (params (WeaponType :type String))
  (returns (Slots :type Integer))
  (locals (`Material Slots` :type "Array of /Game/ModularWeapons/Data/MaterialSlot Enum"))
  (return (`KismetArrayLibrary.Array_Length` (`self.Get MaterialSlots of WeaponType` WeaponType))))

(fn `Get Num Variations for Weapon Part`
  (params (`Weapon Type` :type String) (`Weapon Part Prefix` :type String))
  (returns (NumVariations :type Integer) (`Part found` :type Boolean))
  (locals (`Found Amount` :type Integer) (`Part Type found` :type Boolean) (`Local Weapon Parts` :type "Array of /Game/ModularWeapons/Data/WeaponPart Structure"))
  (bind _output_get (set `local.Local Weapon Parts` (defaults `/Game/ModularWeapons/Data/WeaponData` "/Game/ModularWeapons/Data/WeaponData.WeaponData_C")))
  (for _array_element _output_get
    (bind (_weapontypename _partprefix _meshes) (break `/Game/ModularWeapons/Data/WeaponPart` _array_element))
    (if (== _weapontypename `Weapon Type`)
      (if (== `Weapon Part Prefix` _partprefix)
        (set `local.Part Type found` true)
        (set `local.Found Amount` (`KismetArrayLibrary.Array_Length` _meshes))
        (break))))
  (return (`local.Found Amount`) (`local.Part Type found`)))

(fn `Get Number of Part Categories for Weapon Type`
  (params (`Required Parts` :type Boolean :default false) (`Optional Parts` :type Boolean :default false) (`Weapon Type` :type String))
  (returns (Amount :type Integer))
  (locals (`Amount found` :type Integer) (`Local Weapon Parts` :type "Array of /Game/ModularWeapons/Data/WeaponPart Structure"))
  (bind _output_get (set `local.Local Weapon Parts` (defaults `/Game/ModularWeapons/Data/WeaponData` "/Game/ModularWeapons/Data/WeaponData.WeaponData_C")))
  (for _array_element _output_get
    (bind (_weapontypename _partprefix _meshes _optional) (break `/Game/ModularWeapons/Data/WeaponPart` _array_element))
    (if (== `Weapon Type` _weapontypename)
      (`|ExecutionSequence`
        (:`then_0`
          (if (and `Required Parts` (not _optional))
            (`/Engine/EditorBlueprintResources/StandardMacros.IncrementInt` (`local.Amount found`) :!label _label)))
        (:`then_1`
          (if (and _optional `Optional Parts`)
            (goto _label))))))
  (return (`local.Amount found`)))

(fn `Get Part Index from WeaponCode`
  (params (WeaponCode :type String) (`Weapon Part Prefix` :type String))
  (returns (Index :type Integer))
  (locals (`Found Index` :type Integer))
  (for _array_element (`self.Get Parts from WeaponCode` WeaponCode)
    (if (`KismetStringLibrary.StartsWith` _array_element `Weapon Part Prefix`)
      (`|ExecutionSequence`
        (:`then_0`
          (set `local.Found Index` (`KismetStringLibrary.Conv_StringToInt` (`KismetStringLibrary.RightChop` _array_element (`KismetStringLibrary.Len` `Weapon Part Prefix`)))))
        (:`then_1`
          (break)))))
  (return (`local.Found Index`)))

(fn `Get Parts from WeaponCode`
  (params (WeaponCode :type String))
  (returns (`Weapon Parts` :type "Array of String"))
  (locals (`Output Weapon Parts` :type "Array of String"))
  (set `local.Output Weapon Parts` (`KismetStringLibrary.ParseIntoArray` (`KismetArrayLibrary.Array_Get` (`KismetStringLibrary.ParseIntoArray` WeaponCode ":") 1) "_"))
  (return (`local.Output Weapon Parts`)))

(fn `Get Type from WeaponCode`
  (params (WeaponCode :type String))
  (returns (`Weapon Type` :type String))
  (return (`KismetArrayLibrary.Array_Get` (`KismetStringLibrary.ParseIntoArray` WeaponCode ":"))))

(fn `Get WeaponType`
  (params (`Weapon Type` :type String))
  (returns (`Found Weapon Type` :type "/Game/ModularWeapons/Data/WeaponType Structure") (Success :type Boolean))
  (locals (`Local WeaponType` :type "/Game/ModularWeapons/Data/WeaponType Structure") (`Type found` :type Boolean) (`Local Weapon Types` :type "Array of /Game/ModularWeapons/Data/WeaponType Structure"))
  (bind _output_get (set `local.Local Weapon Types` (`.WeaponTypes` (defaults `/Game/ModularWeapons/Data/WeaponData` "/Game/ModularWeapons/Data/WeaponData.WeaponData_C"))))
  (for _array_element _output_get
    (if (== `Weapon Type` (`.WeaponTypeName_16_DA4B7039464E77528C011C93D37EC128` (break `/Game/ModularWeapons/Data/WeaponType` _array_element)))
      (set `local.Type found` true)
      (set `local.Local WeaponType` _array_element)
      (break)))
  (return (`local.Local WeaponType`) (`local.Type found`)))

(fn `Random Materials Strings of Type`
  (params (`Weapon Type` :type String))
  (returns (`Weapon Materials` :type "Array of String"))
  (locals (`New Materials` :type "Array of String"))
  (for _array_element (`self.Get MaterialSlots of WeaponType` `Weapon Type`)
    (bind (_materialsets _materialsets_shortnames) (`self.Get MaterialSets of Slot` _array_element))
    (`KismetArrayLibrary.Array_Add` (`local.New Materials`) (`KismetArrayLibrary.Array_Get` _materialsets_shortnames (`KismetMathLibrary.RandomInteger` (`KismetArrayLibrary.Array_Length` _materialsets_shortnames)))))
  (return (`local.New Materials`)))

(fn `Random MaterialSet of Slot`
  (params (`Material Slot` :type "/Game/ModularWeapons/Data/MaterialSlot Enum"))
  (returns (`Material Set` :type "/Game/ModularWeapons/Data/MaterialSet Structure") (`Material ShortName` :type String))
  (bind _materialsets (`self.Get MaterialSets of Slot` `Material Slot`))
  (bind _item (`KismetArrayLibrary.Array_Get` _materialsets (`KismetMathLibrary.RandomInteger` (`KismetArrayLibrary.Array_Length` _materialsets))))
  (return _item (`.MaterialUniqueShortName_27_054530BA4E6ABC3F1CEEC68FA6F3C425` (break `/Game/ModularWeapons/Data/MaterialSet` _item))))

(fn `Random Parts Strings of Type`
  (params (`Weapon Type` :type String) (`Optional Parts Weight` :type "Float (double-precision)"))
  (returns (`Weapon Parts` :type "Array of String"))
  (locals (`New Parts` :type "Array of String") (`Local Weapon Parts` :type "Array of /Game/ModularWeapons/Data/WeaponPart Structure") (`Local Filtered Weapon Parts` :type "Array of /Game/ModularWeapons/Data/WeaponPart Structure"))
  (bind _output_get (set `local.Local Weapon Parts` (defaults `/Game/ModularWeapons/Data/WeaponData` "/Game/ModularWeapons/Data/WeaponData.WeaponData_C")))
  (bind _output_get_2 (set `local.Local Filtered Weapon Parts` (`self.Filter Weapon Parts by Type` _output_get `Weapon Type` false `Optional Parts Weight`)))
  (for _array_element _output_get_2
    (bind (_weapontypename _partprefix _meshes) (break `/Game/ModularWeapons/Data/WeaponPart` _array_element))
    (`KismetArrayLibrary.Array_Add` (`local.New Parts`) (`KismetStringLibrary.Concat_StrStr` _partprefix (`KismetStringLibrary.Conv_IntToString` (`KismetMathLibrary.RandomInteger` (`KismetArrayLibrary.Array_Length` _meshes))))))
  (return (`local.New Parts`)))

(fn `Random Weapon Part`
  (params (`Weapon Part` :type "/Game/ModularWeapons/Data/WeaponPart Structure"))
  (returns (PartString :type String))
  (bind (_weapontypename _partprefix _meshes) (break `/Game/ModularWeapons/Data/WeaponPart` `Weapon Part`))
  (return (`KismetStringLibrary.Concat_StrStr` _partprefix (`KismetStringLibrary.Conv_IntToString` (`KismetMathLibrary.RandomInteger` (`KismetArrayLibrary.Array_Length` _meshes))))))

(fn `Random Weapon Type`
  (returns (`Weapon Type` :type String))
  (bind _available_types (`self.Available Weapon Types` null))
  (return (`KismetArrayLibrary.Array_Get` _available_types (`KismetMathLibrary.RandomInteger` (`KismetArrayLibrary.Array_Length` _available_types)))))

(fn `Random WeaponCode (Advanced)`
  (params (`Weapon Code` :type String) (`Optional Parts Weight` :type "Float (double-precision)" :default 0.0) (`Random Type` :type Boolean :default false) (`Random Parts` :type Boolean :default true) (`Random Materials` :type Boolean :default true))
  (returns (WeaponCode :type String))
  (locals (`Filtered Weapon Parts Array` :type "Array of /Game/ModularWeapons/Data/WeaponPart Structure") (`Output String` :type String) (`New Weapon Type` :type String) (`Unfiltered Weapon Parts Array` :type "Array of /Game/ModularWeapons/Data/WeaponPart Structure"))
  ;[1 1 1] Use random or existing type
  (if `Random Type`
    (set `local.Output String` (`self.Random Weapon Type` null))
    (else
      (set `local.Output String` (`self.Get Type from WeaponCode` `Weapon Code`))))
  (bind _output_get (set `local.New Weapon Type` (`local.Output String`)))
  (if `Random Parts`
    (bind _output_get_2 (set `local.Unfiltered Weapon Parts Array` (defaults `/Game/ModularWeapons/Data/WeaponData` "/Game/ModularWeapons/Data/WeaponData.WeaponData_C")))
    ;[1 1 1] Random weapon parts
    (bind _output_get_3 (set `local.Filtered Weapon Parts Array` (`self.Filter Weapon Parts by Type` _output_get_2 _output_get false `Optional Parts Weight`)))
    (for (_array_element _array_index) _output_get_3
      (set `local.Output String` (`KismetStringLibrary.Concat_StrStr` (`local.Output String`) (`KismetMathLibrary.SelectString` ":" "_" (== _array_index 0)) (`self.Random Weapon Part` _array_element))))
    (else
      ;[1 1 1] Use existing parts
      (for (_array_element_2 _array_index_2) (`self.Get Parts from WeaponCode` `Weapon Code`)
        (set `local.Output String` (`KismetStringLibrary.Concat_StrStr` (`local.Output String`) (`KismetMathLibrary.SelectString` ":" "_" (== _array_index_2 0)) _array_element_2)))))
  (if `Random Materials`
    ;[1 1 1] Random materials
    (for (_array_element_3 _array_index_3) (`self.Get MaterialSlots of WeaponType` _output_get)
      (set `local.Output String` (`KismetStringLibrary.Concat_StrStr` (`local.Output String`) (`KismetMathLibrary.SelectString` ":" "_" (== _array_index_3 0)) (`.Material ShortName` (`self.Random MaterialSet of Slot` _array_element_3)))))
    (else
      ;[1 1 1] Use existing materials
      (for (_array_element_4 _array_index_4) (`self.Get Materials from WeaponCode` `Weapon Code`)
        (set `local.Output String` (`KismetStringLibrary.Concat_StrStr` (`local.Output String`) (`KismetMathLibrary.SelectString` ":" "_" (== _array_index_4 0)) _array_element_4)))))
  (return (`local.Output String`)))

(fn `Random WeaponCode of same Type from WeaponCode`
  (params (WeaponCode :type String) (`Optional Parts Weight` :type "Float (double-precision)" :default 0.0))
  (returns (`New WeaponCode` :type String))
  (bind _weaponcode (`self.Random WeaponCode of Type` (`self.Get Type from WeaponCode` WeaponCode) `Optional Parts Weight`))
  (return _weaponcode))

(fn `Random WeaponCode of Type`
  (params (`Weapon Type` :type String) (`Optional Parts Weight` :type "Float (double-precision)" :default 0.0))
  (returns (WeaponCode :type String))
  (locals (`Filtered Weapon Parts Array` :type "Array of /Game/ModularWeapons/Data/WeaponPart Structure") (`Output String` :type String) (`Unfiltered Weapon Parts Array` :type "Array of /Game/ModularWeapons/Data/WeaponPart Structure"))
  (bind _output_get (set `local.Unfiltered Weapon Parts Array` (defaults `/Game/ModularWeapons/Data/WeaponData` "/Game/ModularWeapons/Data/WeaponData.WeaponData_C")))
  (set `local.Output String` `Weapon Type`)
  (bind _output_get_2 (set `local.Filtered Weapon Parts Array` (`self.Filter Weapon Parts by Type` _output_get `Weapon Type` false `Optional Parts Weight`)))
  (for (_array_element _array_index) _output_get_2
    (set `local.Output String` (`KismetStringLibrary.Concat_StrStr` (`local.Output String`) (`KismetMathLibrary.SelectString` ":" "_" (== _array_index 0)) (`self.Random Weapon Part` _array_element))))
  (for (_array_element_2 _array_index_2) (`self.Get MaterialSlots of WeaponType` `Weapon Type`)
    (set `local.Output String` (`KismetStringLibrary.Concat_StrStr` (`local.Output String`) (`KismetMathLibrary.SelectString` ":" "_" (== _array_index_2 0)) (`.Material ShortName` (`self.Random MaterialSet of Slot` _array_element_2)))))
  (return (`local.Output String`)))

(fn `Set Material on WeaponCode`
  (params (WeaponCode :type String) (`Index to set` :type Integer) (`New Material ShortName` :type String))
  (returns (`New WeaponCode` :type String))
  (locals (`Local Materials` :type "Array of String"))
  (bind _output_get (set `local.Local Materials` (`self.Get Materials from WeaponCode` WeaponCode)))
  (`KismetArrayLibrary.Array_Set` _output_get `Index to set` `New Material ShortName`)
  (bind _weaponcode (`self.Compile WeaponCode` (`self.Get Type from WeaponCode` WeaponCode) (`self.Get Parts from WeaponCode` WeaponCode) (`local.Local Materials`)))
  (return _weaponcode))

(fn `Set Part Index on WeaponCode`
  (params (WeaponCode :type String) (`Weapon Part Prefix` :type String) (`New Index` :type Integer))
  (returns (`New WeaponCode` :type String))
  (locals (`New Code` :type String) (`Parts Array` :type "Array of String"))
  (bind _output_get (set `local.Parts Array` (`self.Get Parts from WeaponCode` WeaponCode)))
  (for (_array_element _array_index) _output_get
    (if (`KismetStringLibrary.StartsWith` _array_element `Weapon Part Prefix`)
      (`|ExecutionSequence`
        (:`then_0`
          (`KismetArrayLibrary.Array_Set` _output_get _array_index (`KismetStringLibrary.Concat_StrStr` `Weapon Part Prefix` (`KismetStringLibrary.Conv_IntToString` `New Index`))))
        (:`then_1`
          (break)))))
  (bind _weaponcode (`self.Compile WeaponCode` (`self.Get Type from WeaponCode` WeaponCode) (`local.Parts Array`) (`self.Get Materials from WeaponCode` WeaponCode)))
  (set `local.New Code` _weaponcode)
  (return (`local.New Code`)))