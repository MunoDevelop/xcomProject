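; Clickable in-world button for the modular weapons example that tells a referenced sword spawner to spawn a random weapon.
; The construction script creates a dynamic instance of MI_Button on the button mesh.
; Hover events toggle its Selection parameter, and Interact briefly pulses Clicking as it triggers the spawn.
; Ending hover also clears the Clicking state.
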(event `self.Hover Start`
  (`MaterialInstanceDynamic.SetScalarParameterValue` (`self.Button DMI`) "Selection" 1.0))

(event `self.Hover End`
  (`MaterialInstanceDynamic.SetScalarParameterValue` (`self.Button DMI`) "Selection" 0.0)
  (`MaterialInstanceDynamic.SetScalarParameterValue` (`self.Button DMI`) "Clicking" 0.0))

(event `self.Interact`
  (`|ExecutionSequence`
    (:`then_0`
      (`MaterialInstanceDynamic.SetScalarParameterValue` (`self.Button DMI`) "Clicking" 1.0)
      (`/Game/ModularWeapons/GameExample/Blueprints/RandomSwordSpawner.Spawn Random Weapon` (`self.SwordSpawner Ref`)))
    (:`then_1`
      (`KismetSystemLibrary.Delay` 0.05)
      (`MaterialInstanceDynamic.SetScalarParameterValue` (`self.Button DMI`) "Clicking" 0.0))))

(fn `UserConstructionScript`
  (bind _buttonmesh (`self.ButtonMesh`))
  (bind _returnvalue (`PrimitiveComponent.CreateDynamicMaterialInstance` _buttonmesh 0 "/Game/ModularWeapons/GameExample/Materials/MI_Button.MI_Button"))
  (bind _output_get (set `self.Button DMI` _returnvalue))
  (`PrimitiveComponent.SetMaterial` _buttonmesh 0 _output_get))