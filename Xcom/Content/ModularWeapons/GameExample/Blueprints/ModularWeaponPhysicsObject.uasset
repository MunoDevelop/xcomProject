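; A physics object in the game example that wraps a ModularWeapon child actor in a box Collision component.
; The construction script passes WeaponCode to the child and initializes it, sizes the box to the assembled weapon's bounds, and offsets the mesh to center those bounds on the box.
; On BeginPlay it gives the box a random angular impulse as a velocity change, so the weapon starts with a spin.
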(event `self.ReceiveBeginPlay`
  (`PrimitiveComponent.AddAngularImpulse` (`self.Collision`) (* (`KismetMathLibrary.RandomUnitVector`) 2.0) "None" true))

(fn `UserConstructionScript`
  (bind _asmodular_weapon (cast `/Game/ModularWeapons/Blueprints/ModularWeapon` (`ChildActorComponent.ChildActor` (`self.WeaponMesh`)) :!pure true))
  (bind (_origin _boxextent) (`self.GetActorBounds` _asmodular_weapon false))
  (set `/Game/ModularWeapons/Blueprints/ModularWeapon.WeaponCode` (`self.WeaponCode`) _asmodular_weapon)
  (`/Game/ModularWeapons/Blueprints/ModularWeapon.Initialize` _asmodular_weapon)
  (`BoxComponent.SetBoxExtent` (`self.Collision`) _boxextent true)
  (`SceneComponent.K2_SetRelativeLocation` (`self.WeaponMesh`) (- (`self.K2_GetActorLocation` _asmodular_weapon) _origin) false))