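; RandomSwordSpawner is an actor that spawns randomized modular weapon physics objects at random points inside a box area.
; The construction script sizes the box from SpawnAreaExtents.
; SpawnRandomWeapon builds a weapon code for a random or configured type, then spawns a ModularWeaponPhysicsObject with it, adjusting for collisions, and returns it.
; The event graph has no active logic, so nothing spawns until that function is called.
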(event `self.ReceiveBeginPlay`)

(event `self.ReceiveActorBeginOverlap`
  (params (OtherActor :type "Actor Object Reference")))

(event `self.ReceiveTick`
  (params (DeltaSeconds :type "Float (single-precision)")))

(fn `Spawn Random Weapon`
  (returns (`Spawned Weapon` :type "/Game/ModularWeapons/GameExample/Blueprints/ModularWeaponPhysicsObject Object Reference"))
  (bind _spawnarea (`self.SpawnArea`))
  (bind _weaponcode (`/Game/ModularWeapons/Blueprints/ModularWeaponTools.Random WeaponCode of Type` (`KismetMathLibrary.SelectString` (`/Game/ModularWeapons/Blueprints/ModularWeaponTools.Random Weapon Type`) (`self.Weapon Type`) (`self.Random Weapon Type`)) 0.5))
  (bind _returnvalue (`|SpawnActorFromClass` "/Game/ModularWeapons/GameExample/Blueprints/ModularWeaponPhysicsObject.ModularWeaponPhysicsObject_C" (`KismetMathLibrary.MakeTransform` (`KismetMathLibrary.TransformLocation` (`self.GetTransform`) (`KismetMathLibrary.RandomPointInBoundingBox` (`SceneComponent.RelativeLocation` _spawnarea) (`BoxComponent.BoxExtent` _spawnarea)))) "AdjustIfPossibleButDontSpawnIfColliding" "OverrideRootScale" null _weaponcode))
  (return _returnvalue))

(fn `UserConstructionScript`
  (`BoxComponent.SetBoxExtent` (`self.SpawnArea`) (`self.SpawnAreaExtents`) true))